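; BP_GameManager is a game manager that, after the game starts, enables player overlap and plays a recurring sound.
; Tick waits a minute once GameStarted is set, then sets CanOverlap on player 0's BP_MyPlayer and latches Called.
; A looping Delay re-arms a short timer every ten seconds to play Khalnayak at ServerLocation.
; Separate authority-only and client sound functions, gated by ShouldPlaySound, are not called within this Blueprint.
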(event Custom|PlaySound
  (Audio|PlaySoundatLocation "/Game/Audios/Khalnayak.Khalnayak" (Variables|Default|GetServerLocation) "0, 0, 0" 1.0 1.0 0.0 "/Game/Sounds/ATT_Voip.ATT_Voip" 0 0 0))

(event EventBeginPlay)

(event Collision|EventActorBeginOverlap
  (params (OtherActor :type Actor%20Object%20Reference)))

(event EventTick
  (params (DeltaSeconds :type Float%20%28single-precision%29))
  (if (and (Variables|Default|GetGameStarted) (not (Variables|Default|Getcalled)))
    (Utilities|FlowControl|Delay 6e+01)
    (bind _asbp_my_player (Utilities|Casting|CastToBP_MyPlayer (Game|Player|GetPlayerPawn 0)))
    (Variables|/Script/ServerIsTagger.PlayerCharacter|SetbCanOverlap _asbp_my_player true)
    (Utilities|Time|SetTimerbyEvent (delegate Custom|PlaySound) 0.1 :!label _label)
    (Variables|Default|Setcalled true)
    (Utilities|FlowControl|Delay 1e+01)
    (goto _label)))

(fn ConstructionScript)

(fn PlaySoundatServer
  (Networking|SwitchHasAuthority
    (:Authority
      (if (Variables|Default|GetShouldPlaySound)
        (Audio|PlaySoundatLocation "/Game/Audios/Khalnayak.Khalnayak" "0, 0, 0" "0, 0, 0" 1.0 1.0 0.0 "/Game/Sounds/ATT_Voip.ATT_Voip" 0 0 0)))))

(fn PlaySoundatServerClient
  (if (Variables|Default|GetShouldPlaySound)
    (Audio|PlaySoundatLocation "/Game/Audios/Khalnayak.Khalnayak" "0, 0, 0" "0, 0, 0" 1.0 1.0 0.0 0 0 0 0)))