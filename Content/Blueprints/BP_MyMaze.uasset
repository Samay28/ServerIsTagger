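; BP_MyMaze is a maze actor with a start-controlled Barrier and a FinalBox trigger.
; Every tick it looks up BP_GameManager and, while GameStarted is true, turns off the Barrier's collision.
; When player character 0 enters FinalBox, that character's input is disabled, only on the Remote (non-authority) branch.
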(event OnComponentBeginOverlap(FinalBox)
  (params (OverlappedComponent :type Primitive%20Component%20Object%20Reference) (OtherActor :type Actor%20Object%20Reference) (OtherComp :type Primitive%20Component%20Object%20Reference) (OtherBodyIndex :type Integer) (bFromSweep :type Boolean) (SweepResult :type Hit%20Result%20Structure%20%28by%20ref%29))
  (bind _returnvalue (Game|GetPlayerCharacter 0))
  (if (== OtherActor _returnvalue)
    (Networking|SwitchHasAuthority
      (:Remote
        (Input|DisableInput _returnvalue 0)))))

(event Custom|CollisionBarrier
  (Collision|SetCollisionEnabled (Variables|Default|GetBarrier) "NoCollision"))

(event EventBeginPlay)

(event Collision|EventActorBeginOverlap
  (params (OtherActor :type Actor%20Object%20Reference)))

(event EventTick
  (params (DeltaSeconds :type Float%20%28single-precision%29))
  (bind _returnvalue (Actor|GetActorOfClass "/Game/Blueprints/BP_GameManager.BP_GameManager_C"))
  (if (Variables|/Script/ServerIsTagger.GameManager|GetGameStarted _returnvalue)
    (CallFunction|CollisionBarrier)))

(fn ConstructionScript)