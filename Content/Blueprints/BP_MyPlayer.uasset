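; Player Blueprint handling footstep audio, teleport input, a local HUD and a Tab-toggled control panel.
; Tick plays the footstep timeline while moving and sprint input doubles its rate.
; The timeline's Footsteps track calls FootstepTry, which plays an attenuated sound if a downward sphere trace hits.
; Authority switches limit teleport calls to the remote side and control panel opening to the server.
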(event Custom|AddWidget
  (if (Pawn|IsLocallyControlled)
    (bind _returnvalue (UserInterface|CreateWidget "/Game/UI/WBP_MainHud.WBP_MainHud_C" (Game|GetPlayerController 0)))
    (UserInterface|Viewport|AddtoViewport _returnvalue 0)))

(event Input|EnhancedActionEvents|EnhancedInputActionIA_Teleport
  (params (ActionValue :type Boolean) (ElapsedSeconds :type Float%20%28double-precision%29) (TriggeredSeconds :type Float%20%28double-precision%29) (InputAction :type Input%20Action%20Object%20Reference :default "/Game/Inputs/IA_Teleport.IA_Teleport"))
  (:Completed
    (Networking|SwitchHasAuthority
      (:Remote
        (Class|PlayerCharacter|TeleportPlayer)))))

(event Input|EnhancedActionEvents|EnhancedInputActionIA_Sprint
  (params (ActionValue :type Boolean) (ElapsedSeconds :type Float%20%28double-precision%29) (TriggeredSeconds :type Float%20%28double-precision%29) (InputAction :type Input%20Action%20Object%20Reference :default "/Game/Inputs/IA_Sprint.IA_Sprint"))
  (:Triggered
    (Components|Timeline|SetPlayRate (Variables|Default|GetFootsteps_TL) 2.0))
  (:Completed
    (Components|Timeline|SetPlayRate (Variables|Default|GetFootsteps_TL) 1.0)))

(event Collision|EventActorBeginOverlap
  (params (OtherActor :type Actor%20Object%20Reference)))

(event EventTick
  (params (DeltaSeconds :type Float%20%28single-precision%29))
  (bind _footsteps_tl (Variables|Default|GetFootsteps_TL))
  (if (> (Math|Vector|VectorLength (Transformation|GetVelocity)) 0.0)
    (Audio|Components|Audio|Play _footsteps_tl)
    (else
      (Audio|Components|Audio|Stop _footsteps_tl))))

(event Input|KeyboardEvents|Tab
  (params (Key :type Key%20Structure :default "None"))
  (bind _returnvalue (Game|GetPlayerController 0))
  (:Pressed
    (if (Variables|Default|GetIsControlPanelOpened)
      (Widget|RemovefromParent (stale _returnvalue_2))
      (Variables|/Script/Engine.PlayerController|SetbShowMouseCursor _returnvalue false)
      (Variables|Default|SetIsControlPanelOpened false)
      (else
        (Networking|SwitchHasAuthority
          (:Authority
            (bind _returnvalue_2 (UserInterface|CreateWidget "/Game/UI/WBP_ControlPanel.WBP_ControlPanel_C"))
            (UserInterface|Viewport|AddtoViewport _returnvalue_2 0)
            (Variables|Default|SetIsControlPanelOpened true)
            (Variables|/Script/Engine.PlayerController|SetbShowMouseCursor _returnvalue true)))))))

(fn ConstructionScript)

(fn TraceFootsteps
  (bind _returnvalue (Transformation|GetActorLocation))
  (bind _capsulecomponent (Variables|Default|GetCapsuleComponent))
  (bind (_x _y _z) (Class|KismetMathLibrary|BreakVector3f _returnvalue))
  (bind _returnvalue_2 (Collision|SphereTraceByChannel _returnvalue (Math|Vector|MakeVector _x _y (- _z (Components|Capsule|GetScaledCapsuleHalfHeight _capsulecomponent))) (Components|Capsule|GetScaledCapsuleRadius _capsulecomponent) "TraceTypeQuery1" false 0 "None"))
  (return _returnvalue_2))

(fn FootstepTry
  (bind _finished (CallFunction|TraceFootsteps))
  (if _finished
    (Audio|PlaySoundatLocation "/Game/Audios/FootstepsCue.FootstepsCue" (Transformation|GetActorLocation) "0, 0, 0" 1.0 1.0 0.0 "/Game/Sounds/ATT_Voip.ATT_Voip" 0 0 0)))