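; Player Blueprint that sets up positional voice chat for itself.
; On BeginPlay it adds a VOIP Talker component, then polls on a short delay until its PlayerState is valid.
; It then registers the talker with that PlayerState, sets the mic threshold, and attaches the voice to the Mesh with the ATT_Voip attenuation asset.
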(event EventBeginPlay
  (bind _playerstate (Variables|Default|GetPlayerState))
  (bind _returnvalue (AddComponent|AddVOIPTalker))
  (bind _output_get (Variables|Default|SetVoipRef _returnvalue))
  (Utilities|IsValid _playerstate :!label _label
    (:Is%20Valid
      (Class|VOIPTalker|RegisterwithPlayerState _output_get _playerstate)
      (Class|VOIPStatics|SetMicThreshold -1.0)
      (Variables|/Script/Engine.VOIPTalker|SetSettings (Variables|Default|GetVoipRef) (Utilities|Struct|MakeVoiceSettings (Variables|Character|GetMesh) "/Game/Sounds/ATT_Voip.ATT_Voip")))
    (:Is%20Not%20Valid
      (Utilities|FlowControl|Delay 0.2)
      (goto _label))))

(event Collision|EventActorBeginOverlap
  (params (OtherActor :type Actor%20Object%20Reference)))

(event EventTick
  (params (DeltaSeconds :type Float%20%28single-precision%29)))

(fn ConstructionScript)